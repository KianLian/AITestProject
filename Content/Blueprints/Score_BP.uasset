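; Score_BP is a pickup that adds points to a Character_BP when its Capsule overlaps that character's capsule component, then destroys itself after a short delay.
; An outer Sphere overlap starts a fast looping timer if the character's Magnet flag is on.
; Each tick of that timer uses VInterpTo to pull the pickup toward the overlapping actor, and any Sphere end overlap clears it.
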(event OnComponentBeginOverlap(Capsule)
  (params (OverlappedComponent :type Primitive%20Component%20Object%20Reference) (OtherActor :type Actor%20Object%20Reference) (OtherComp :type Primitive%20Component%20Object%20Reference) (OtherBodyIndex :type Integer) (bFromSweep :type Boolean) (SweepResult :type Hit%20Result%20Structure%20%28by%20ref%29))
  (bind _ascharacter_bp (Utilities|Casting|CastToCharacter_BP OtherActor))
  (if (== OtherComp (Variables|/Script/Engine.Character|GetCapsuleComponent _ascharacter_bp))
    (Default|AddPoints _ascharacter_bp (Variables|Default|GetPoints))
    (Utilities|FlowControl|Delay 0.2)
    (Actor|DestroyActor)))

(event OnComponentBeginOverlap(Sphere)
  (params (OverlappedComponent :type Primitive%20Component%20Object%20Reference) (OtherActor :type Actor%20Object%20Reference) (OtherComp :type Primitive%20Component%20Object%20Reference) (OtherBodyIndex :type Integer) (bFromSweep :type Boolean) (SweepResult :type Hit%20Result%20Structure%20%28by%20ref%29))
  (bind _ascharacter_bp (Utilities|Casting|CastToCharacter_BP OtherActor))
  (if (Variables|/Game/Character/Character_BP.Character_BP_C|GetMagnet _ascharacter_bp)
    (bind _returnvalue (Utilities|Time|SetTimerbyEvent (delegate Custom|Move) 0.01 true))))

(event OnComponentEndOverlap(Sphere)
  (params (OverlappedComponent :type Primitive%20Component%20Object%20Reference) (OtherActor :type Actor%20Object%20Reference) (OtherComp :type Primitive%20Component%20Object%20Reference) (OtherBodyIndex :type Integer))
  (Utilities|Time|ClearandInvalidateTimerbyHandle (stale OnComponentBeginOverlap(Sphere) _returnvalue)))

(event Custom|Move
  (Transformation|SetWorldLocation (Variables|Default|GetDefaultSceneRoot) (Math|Interpolation|VInterpTo (Transformation|GetActorLocation) (Transformation|GetActorLocation (stale OnComponentBeginOverlap(Sphere) OtherActor)) 0.05 (Variables|Default|GetInterp%20Speed)) false false))

(fn ConstructionScript)