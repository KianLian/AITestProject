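; Torch actor with a FireLight effect and a point light that other logic can ignite.
; The construction script tints the point light with a LightColor variable and starts it hidden.
; The SetLight event passes its Pressed flag to both components, but only while FireLight is inactive, so a lit torch cannot be switched off through it.
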(event EventBeginPlay)

(event Collision|EventActorBeginOverlap
  (params (OtherActor :type Actor%20Object%20Reference)))

(event EventTick
  (params (DeltaSeconds :type Float%20%28single-precision%29)))

(event EventSetLight
  (params (Pressed :type Boolean))
  (bind _firelight (Variables|Default|GetFireLight))
  (if (not (Components|Activation|IsActive _firelight))
    (Components|Activation|SetActive _firelight Pressed false)
    (Rendering|SetVisibility (Variables|Default|GetPointLight) Pressed false)))

(fn ConstructionScript
  (bind _pointlight (Variables|Default|GetPointLight))
  (Rendering|Components|Light|SetLightColor _pointlight (Variables|Default|GetLightColor) true)
  (Rendering|SetVisibility _pointlight false false))