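; Fruit pickup that restores the Character_BP's life and destroys itself when it touches that character's capsule while life is below 100.
; An outer Sphere acts as a magnet range: if the character's Magnet flag is on and life is below 100, it starts a fast looping timer.
; Each tick interpolates the fruit toward the overlapping actor, and any end overlap on the Sphere clears the timer.
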(event OnComponentBeginOverlap(Capsule)
  (params (OverlappedComponent :type Primitive%20Component%20Object%20Reference) (OtherActor :type Actor%20Object%20Reference) (OtherComp :type Primitive%20Component%20Object%20Reference) (OtherBodyIndex :type Integer) (bFromSweep :type Boolean) (SweepResult :type Hit%20Result%20Structure%20%28by%20ref%29))
  (bind _ascharacter_bp (Utilities|Casting|CastToCharacter_BP OtherActor))
  (if (and (< (Variables|/Game/Character/Character_BP.Character_BP_C|GetLife _ascharacter_bp) 1e+02) (== OtherComp (Variables|/Script/Engine.Character|GetCapsuleComponent _ascharacter_bp)))
    (Default|RegainLife _ascharacter_bp (Variables|Default|GetHpw%20Much%20Life))
    (Actor|DestroyActor)))

(event OnComponentBeginOverlap(Sphere)
  (params (OverlappedComponent :type Primitive%20Component%20Object%20Reference) (OtherActor :type Actor%20Object%20Reference) (OtherComp :type Primitive%20Component%20Object%20Reference) (OtherBodyIndex :type Integer) (bFromSweep :type Boolean) (SweepResult :type Hit%20Result%20Structure%20%28by%20ref%29))
  (bind _ascharacter_bp (Utilities|Casting|CastToCharacter_BP OtherActor))
  (if (and (Variables|/Game/Character/Character_BP.Character_BP_C|GetMagnet _ascharacter_bp) (< (Variables|/Game/Character/Character_BP.Character_BP_C|GetLife _ascharacter_bp) 1e+02))
    (bind _returnvalue (Utilities|Time|SetTimerbyEvent (delegate Custom|Move) 0.01 true))))

(event OnComponentEndOverlap(Sphere)
  (params (OverlappedComponent :type Primitive%20Component%20Object%20Reference) (OtherActor :type Actor%20Object%20Reference) (OtherComp :type Primitive%20Component%20Object%20Reference) (OtherBodyIndex :type Integer))
  (Utilities|Time|ClearandInvalidateTimerbyHandle (stale OnComponentBeginOverlap(Sphere) _returnvalue)))

(event Custom|Move
  (Transformation|SetWorldLocation (Variables|Default|GetDefaultSceneRoot) (Math|Interpolation|VInterpTo (Transformation|GetActorLocation) (Transformation|GetActorLocation (stale OnComponentBeginOverlap(Sphere) OtherActor)) 0.05 (Variables|Default|GetInterp%20Speed)) false false))

(fn ConstructionScript)