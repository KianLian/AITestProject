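; Bush actor that changes appearance after enough exposure to flame.
; CollidesFlame starts a one-second timer on MenosTimes, using the Colliding flag as its looping setting.
; Each tick of that timer increments a Time counter, which is never reset here.
; When the counter equals five, ChangeColor swaps the static mesh's first material to a concrete tiles material.
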(event Custom|MenosTimes
  (bind _output_get (Variables|Default|SetTime (+ (Variables|Default|GetTime) 1.0)))
  (if (== _output_get 5.0)
    (CallFunction|ChangeColor)))

(event EventBeginPlay)

(event Collision|EventActorBeginOverlap
  (params (OtherActor :type Actor%20Object%20Reference)))

(event EventTick
  (params (DeltaSeconds :type Float%20%28single-precision%29)))

(event EventCollidesFlame
  (params (Colliding :type Boolean))
  (Utilities|Time|SetTimerbyEvent (delegate Custom|MenosTimes) 1.0 Colliding))

(fn ConstructionScript)

(fn ChangeColor
  (Rendering|Material|SetMaterial (Variables|Default|GetStaticMesh) 0 "/Game/StarterContent/Materials/M_Concrete_Tiles.M_Concrete_Tiles"))