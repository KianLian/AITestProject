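; Portal actor that ends a level when the player's Character_BP capsule enters its Box trigger.
; On a normal level it opens the level named by LevelName.
; When LastLevel is set, it instead shows the CompletedGame widget, pauses the game and enables the mouse cursor with Game and UI input focused on the widget.
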(event OnComponentBeginOverlap(Box)
  (params (OverlappedComponent :type Primitive%20Component%20Object%20Reference) (OtherActor :type Actor%20Object%20Reference) (OtherComp :type Primitive%20Component%20Object%20Reference) (OtherBodyIndex :type Integer) (bFromSweep :type Boolean) (SweepResult :type Hit%20Result%20Structure%20%28by%20ref%29))
  (bind _returnvalue (Game|GetPlayerController 0))
  (bind _ascharacter_bp (Utilities|Casting|CastToCharacter_BP OtherActor))
  (if (== OtherComp (Variables|/Script/Engine.Character|GetCapsuleComponent _ascharacter_bp))
    (if (Variables|Default|GetLastLevel?)
      (bind _returnvalue_2 (UserInterface|CreateWidget "/Game/Widgets/CompletedGame.CompletedGame_C"))
      (UserInterface|Viewport|AddtoViewport _returnvalue_2 0)
      (Game|SetGamePaused true)
      (Variables|/Script/Engine.PlayerController|SetbShowMouseCursor _returnvalue true)
      (Input|SetInputModeGameandUI _returnvalue _returnvalue_2 "DoNotLock" false)
      (else
        (Game|OpenLevel(byName) (Variables|Default|GetLevel%20Name))))))

(event EventBeginPlay)

(event Collision|EventActorBeginOverlap
  (params (OtherActor :type Actor%20Object%20Reference)))

(event EventTick
  (params (DeltaSeconds :type Float%20%28single-precision%29)))

(fn ConstructionScript)