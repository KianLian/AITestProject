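; Rocks_BP is a rock Blueprint that switches on its particle system after accumulated flame contact.
; CollidesFlame sets a one-second timer, using its Colliding flag as the looping setting, so a false call still leaves a single tick pending.
; Each tick increments a Time counter, which is never reset here, and calls SetParticles to activate the particles when it equals five.
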(event Custom|MenosTimes
  (bind _output_get (Variables|Default|SetTime (+ (Variables|Default|GetTime) 1.0)))
  (if (== _output_get 5.0)
    (CallFunction|SetParticles)))

(event EventBeginPlay)

(event Collision|EventActorBeginOverlap
  (params (OtherActor :type Actor%20Object%20Reference)))

(event EventTick
  (params (DeltaSeconds :type Float%20%28single-precision%29)))

(event EventCollidesFlame
  (params (Colliding :type Boolean))
  (Utilities|Time|SetTimerbyEvent (delegate Custom|MenosTimes) 1.0 Colliding))

(fn ConstructionScript)

(fn SetParticles
  (Components|Activation|SetActive (Variables|Default|GetParticleSystem) true false))