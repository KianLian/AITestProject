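; ManaPool is a pickup-area actor that refills the mana of a Character_BP while it stands inside the pool's Box.
; Beginning overlap starts a looping 0.1-second timer that calls RegenMana on the overlapping character while its mana is not full.
; The regen tick also activates RotatingMovement.
; Ending overlap stops the rotation and clears the timer.
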(event OnComponentBeginOverlap(Box)
  (params (OverlappedComponent :type Primitive%20Component%20Object%20Reference) (OtherActor :type Actor%20Object%20Reference) (OtherComp :type Primitive%20Component%20Object%20Reference) (OtherBodyIndex :type Integer) (bFromSweep :type Boolean) (SweepResult :type Hit%20Result%20Structure%20%28by%20ref%29))
  (bind _output_get (Variables|Default|SetPlayerColliding true))
  (bind _returnvalue (Utilities|Time|SetTimerbyEvent (delegate Custom|ManaPoool) 0.1 _output_get)))

(event OnComponentEndOverlap(Box)
  (params (OverlappedComponent :type Primitive%20Component%20Object%20Reference) (OtherActor :type Actor%20Object%20Reference) (OtherComp :type Primitive%20Component%20Object%20Reference) (OtherBodyIndex :type Integer))
  (bind _output_get (Variables|Default|SetPlayerColliding false))
  (Components|Activation|SetActive (Variables|Default|GetRotatingMovement) _output_get false)
  (Utilities|Time|ClearandInvalidateTimerbyHandle (stale OnComponentBeginOverlap(Box) _returnvalue)))

(event Custom|ManaPoool
  (bind _ascharacter_bp (Utilities|Casting|CastToCharacter_BP (stale OnComponentBeginOverlap(Box) OtherActor)))
  (if (and (Variables|Default|GetPlayerColliding) (not (Variables|/Game/Character/Character_BP.Character_BP_C|GetManaFull _ascharacter_bp)))
    (Default|RegenMana _ascharacter_bp (Variables|Default|GetMana))
    (Components|Activation|SetActive (Variables|Default|GetRotatingMovement) (and (Variables|Default|GetPlayerColliding) (not (Variables|/Game/Character/Character_BP.Character_BP_C|GetManaFull _ascharacter_bp))) false)))

(fn ConstructionScript)